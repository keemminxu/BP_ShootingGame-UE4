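; BP_Enemy is a shooter enemy that fires one BP_EnemyBullet on spawn and flies in a fixed direction.
; BeginPlay picks that direction at random, either straight down or toward BP_Player's position, defaulting to down without a player, and Tick moves it with sweep.
; Sphere overlap plays explosion effects and destroys both actors.
; If the other actor's name contains "Player", EndGame also pauses and shows WBP_Menu with the cursor.
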(event OnComponentBeginOverlap(Sphere)
  (params (OverlappedComponent :type Primitive%20Component%20Object%20Reference) (OtherActor :type Actor%20Object%20Reference) (OtherComp :type Primitive%20Component%20Object%20Reference) (OtherBodyIndex :type Integer) (bFromSweep :type Boolean) (SweepResult :type Hit%20Result%20Structure%20%28by%20ref%29))
  ;[1 1 1] 다른 물체와 부딪혔을 때 호출되는 이벤트
  ;[1 1 1] 폭발효과 만들기
  (Effects|SpawnEmitteratLocation "/Game/StarterContent/Particles/P_Explosion.P_Explosion" (Transformation|GetActorLocation))
  (Audio|PlaySound2D "/Game/Sounds/Audio_Explosion.Audio_Explosion" 1.0 1.0 0.0 0 0)
  ;[1 1 1] 부딪힌 대상이 Player 인지 검출
  (if (Utilities|String|Contains (Utilities|GetObjectName OtherActor) "Player")
    (CallFunction|EndGame))
  ;[1 1 1] 같이 죽겠다
  (Actor|DestroyActor OtherActor)
  (Actor|DestroyActor))

(event EventTick
  (params (DeltaSeconds :type Float%20%28single-precision%29))
  ;[1 1 1] P= P0 * Vt 이동한다
  ;;[1 1 1] t
  ;;[1 1 1] P
  (Transformation|SetActorLocation (+ (Transformation|GetActorLocation) (* (* (Variables|Default|GetDirection) (Variables|Default|GetSpeed)) DeltaSeconds)) true false))

(event EventBeginPlay
  (Game|SpawnActorfromClass "/Game/Blueprint/BP_EnemyBullet.BP_EnemyBullet_C" (Transformation|GetWorldTransform (Variables|Default|GetFirePosition)) "Undefined" 0 0)
  (bind _returnvalue (Actor|GetActorOfClass "/Game/Blueprint/BP_Player.BP_Player_C"))
  (bind _output_get (Variables|Default|SetTarget _returnvalue))
  ;[1 1 1] 랜덤하게
  ;;[1 1 1] 50% 미만인지 검사
  (if (Utilities|IsValid _output_get)
    (if (< (Math|Random|RandomIntegerinRange 1 100) 51)
      (Variables|Default|SetDirection "0, 0,-1.000000")
      (else
        (Variables|Default|SetDirection (Math|Vector|Normalize (- (Transformation|GetActorLocation (Variables|Default|GetTarget)) (Transformation|GetActorLocation))))))
    (else
      (Variables|Default|SetDirection "0, 0,-1.000000"))))

(fn ConstructionScript)

(fn EndGame
  (Game|SetGamePaused true)
  (Variables|/Script/Engine.PlayerController|SetbShowMouseCursor (Game|GetPlayerController 0) true)
  (bind _returnvalue (UserInterface|CreateWidget "/Game/UI/WBP_Menu.WBP_Menu_C"))
  (UserInterface|Viewport|AddtoViewport _returnvalue 0))