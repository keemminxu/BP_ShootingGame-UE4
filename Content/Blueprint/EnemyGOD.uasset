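; EnemyGOD is a spawner actor that keeps creating BP_Enemy instances at its own transform.
; On BeginPlay it starts a looping timer by function name that calls CreateEnemy every CreateTime.
; An older elapsed-time counter that called the same function is left disconnected in the event graph and never runs.
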(event EventBeginPlay
  (Utilities|Time|SetTimerbyFunctionName 0 "CreateEnemy" (Variables|Default|GetCreateTime) true))

(event Collision|EventActorBeginOverlap
  (params (OtherActor :type Actor%20Object%20Reference)))

(event EventTick
  (params (DeltaSeconds :type Float%20%28single-precision%29)))

(fn ConstructionScript)

(fn CreateEnemy
  ;[1 1 1] 적을 만들고 싶다
  (Game|SpawnActorfromClass "/Game/Blueprint/BP_Enemy.BP_Enemy_C" (Transformation|GetActorTransform) "Undefined" 0 0))