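; BP_EnemyBullet is an enemy projectile that moves straight down along world -Z at Speed, using a swept, delta-time-scaled move each Tick.
; When its Box begins an overlap, it spawns an explosion effect, plays a sound and destroys the other actor without filtering or destroying itself.
; Disconnected nodes hold an unfinished 50% choice between falling and homing on BP_Player, so that logic never runs.
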(event OnComponentBeginOverlap(Box)
  (params (OverlappedComponent :type Primitive%20Component%20Object%20Reference) (OtherActor :type Actor%20Object%20Reference) (OtherComp :type Primitive%20Component%20Object%20Reference) (OtherBodyIndex :type Integer) (bFromSweep :type Boolean) (SweepResult :type Hit%20Result%20Structure%20%28by%20ref%29))
  (Effects|SpawnEmitteratLocation "/Game/StarterContent/Particles/P_Explosion.P_Explosion" (Transformation|GetActorLocation))
  (Audio|PlaySound2D "/Game/Sounds/Audio_Explosion.Audio_Explosion" 1.0 1.0 0.0 0 0)
  (Actor|DestroyActor OtherActor))

(event EventTick
  (params (DeltaSeconds :type Float%20%28single-precision%29))
  ;[1 1 1] 아래로 이동하고싶다
  (Transformation|SetActorLocation (+ (Transformation|GetActorLocation) (* (Math|Vector|Normalize (Math|Vector|MakeVector 0.0 0.0 -1.0)) (* DeltaSeconds (Variables|Default|GetSpeed)))) true false))

(event EventBeginPlay
  ;[1 1 1] 50% 미만인지 검사
)

(fn ConstructionScript)