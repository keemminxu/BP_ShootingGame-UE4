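; Player actor for a shooter that moves in the Y-Z plane and fires bullets.
; Axis inputs and arrow keys both set integer Horizontal and Vertical values, which Tick normalizes into a swept, frame-rate independent move scaled by Speed.
; The Fire action or F key spawns BP_Bullet at FirePosition and plays a 2D sound.
; Separate per-axis movement nodes remain in the graph but never run.
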(event EventBeginPlay
  (Input|EnableInput (Game|GetPlayerController 0)))

(event EventTick
  (params (DeltaSeconds :type Float%20%28single-precision%29))
  ;[1 1 1] 이동하고싶다
  (Transformation|SetActorLocation (+ (Transformation|GetActorLocation) (* (Math|Vector|Normalize (Math|Vector|MakeVector 0.0 (Math|Conversions|ToFloat(Integer) (Variables|Default|GetHorizontal)) (Math|Conversions|ToFloat(Integer) (Variables|Default|GetVertical)))) (* DeltaSeconds (Variables|Default|GetSpeed)))) true false))

(event Input|ActionEvents|InputActionFire
  (params (Key :type Key%20Structure :default "None"))
  ;[1 1 1] 총알 발사
  (:Pressed
    (Game|SpawnActorfromClass "/Game/Blueprint/BP_Bullet.BP_Bullet_C" (Transformation|GetWorldTransform (Variables|Default|GetFirePosition)) "Undefined" 0 0)
    (Audio|PlaySound2D "/Game/Sounds/Audio_Bullet.Audio_Bullet" 1.0 1.0 0.0 0 0)))

(event Input|AxisEvents|InputAxisHorizontal
  (params (AxisValue :type Float%20%28single-precision%29))
  ;[1 1 1] 입력을 받아서 방향을 구한다
  (Variables|Default|SetHorizontal (Math|Float|Truncate AxisValue)))

(event Input|AxisEvents|InputAxisVertical
  (params (AxisValue :type Float%20%28single-precision%29))
  ;[1 1 1] 입력을 받아서 방향을 구한다
  (Variables|Default|SetVertical (Math|Float|Truncate AxisValue)))

(event Input|KeyboardEvents|Left
  (params (Key :type Key%20Structure :default "None"))
  ;[1 1 1] 수평입력처리
  (:Pressed
    (Variables|Default|SetHorizontal -1))
  (:Released
    (Variables|Default|SetHorizontal 0)))

(event Input|KeyboardEvents|Right
  (params (Key :type Key%20Structure :default "None"))
  ;[1 1 1] 수평입력처리
  (:Pressed
    (Variables|Default|SetHorizontal 1))
  (:Released
    (Variables|Default|SetHorizontal 0)))

(event Input|KeyboardEvents|Up
  (params (Key :type Key%20Structure :default "None"))
  ;[1 1 1] 수직입력처리
  (:Pressed
    (Variables|Default|SetVertical 1))
  (:Released
    (Variables|Default|SetVertical 0)))

(event Input|KeyboardEvents|Down
  (params (Key :type Key%20Structure :default "None"))
  ;[1 1 1] 수직입력처리
  (:Pressed
    (Variables|Default|SetVertical -1))
  (:Released
    (Variables|Default|SetVertical 0)))

(event Input|KeyboardEvents|F
  (params (Key :type Key%20Structure :default "None"))
  ;[1 1 1] 총알 발사
  (:Pressed
    (Game|SpawnActorfromClass "/Game/Blueprint/BP_Bullet.BP_Bullet_C" (Transformation|GetWorldTransform (Variables|Default|GetFirePosition)) "Undefined" 0 0)
    (Audio|PlaySound2D "/Game/Sounds/Audio_Bullet.Audio_Bullet" 1.0 1.0 0.0 0 0)))

(fn ConstructionScript)